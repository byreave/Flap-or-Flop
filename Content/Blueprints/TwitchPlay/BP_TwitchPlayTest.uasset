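; Test Blueprint for Twitch chat control that lets viewers move the current tile and change its gap.
; BeginPlay uses the OAuth token, username and channel to connect and authenticate the TwitchPlay component, printing any failure.
; It then registers Up, Down, Inflate and Deflate chat commands, whose callbacks act on CurrentTile.
; The missing-token warning, chat echo and SPAWN registration are unwired and never run.
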(event `self.ReceiveBeginPlay`
  (bind _twitchplay (`self.TwitchPlay`))
  (bind _oauth_token (`self.oauth_token`))
  ;[1 1 1] Initial Setup
  (if (not (`KismetStringLibrary.EqualEqual_StrStr` _oauth_token))
    (`TwitchIRCComponent.SetUserInfo` _twitchplay _oauth_token (`self.username`) (`self.channel`))
    (bind (__out_error _returnvalue) (`TwitchIRCComponent.Connect` _twitchplay))
    (if _returnvalue
      (bind (__out_error_2 _returnvalue_2) (`TwitchIRCComponent.AuthenticateTwitchIRC` (`self.TwitchPlay`)))
      (if _returnvalue_2
        ;[1 1 1] Registering custom events from chat
        (`TwitchPlayComponent.SetupEncapsulationChars` (`self.TwitchPlay`) "!" "#")
        ;[1 1 1] Up
        (`TwitchPlayComponent.RegisterCommand` (`self.TwitchPlay`) "Up" (delegate `EventMovesUp`))
        ;[1 1 1] Down
        (`TwitchPlayComponent.RegisterCommand` (`self.TwitchPlay`) "Down" (delegate `MoveDown`))
        ;[1 1 1] Inflate
        (`TwitchPlayComponent.RegisterCommand` (`self.TwitchPlay`) "Inflate" (delegate `Inflate`))
        ;[1 1 1] Deflate
        (`TwitchPlayComponent.RegisterCommand` (`self.TwitchPlay`) "Deflate" (delegate `Deflate`))
        (else
          (`self.PrintError` __out_error_2)))
      (else
        (`self.PrintError` __out_error)))))

(event `Event Spawn`
  (params (_command_name :type String) (_command_options :type "Array of String (by ref)") (_sender_username :type String))
  ;[1 1 1] Registering custom events from chat
  (`self.PrintMessage` "SpawnDetected"))

(event `self.TwitchPlay.OnMessageReceived`
  (params (_message :type String) (_username :type String))
  ;[1 1 1] Receiving messages from chat
)

(event `EventMovesUp`
  (params (_command_name :type String) (_command_options :type "Array of String (by ref)") (_sender_username :type String))
  ;[1 1 1] Up
  (`/Game/Blueprints/ByreaveBP_Tile.MovesUp` (`self.CurrentTile`)))

(event `Inflate`
  (params (_command_name :type String) (_command_options :type "Array of String (by ref)") (_sender_username :type String))
  ;[1 1 1] Inflate
  (`/Game/Blueprints/ByreaveBP_Tile.InflateGap` (`self.CurrentTile`)))

(event `MoveDown`
  (params (_command_name :type String) (_command_options :type "Array of String (by ref)") (_sender_username :type String))
  ;[1 1 1] Down
  (`/Game/Blueprints/ByreaveBP_Tile.MovesDown` (`self.CurrentTile`)))

(event `Deflate`
  (params (_command_name :type String) (_command_options :type "Array of String (by ref)") (_sender_username :type String))
  ;[1 1 1] Deflate
  (`/Game/Blueprints/ByreaveBP_Tile.DeflateGap` (`self.CurrentTile`)))

(fn `PrintError`
  (params (error :type String))
  (`KismetSystemLibrary.PrintString` error true true (struct :`R` 1.0 :`B` 0.06219 :`A` 1.0) 10.0)
  (return))

(fn `PrintMessage`
  (params (message :type String))
  (`KismetSystemLibrary.PrintString` message true true (struct :`R` 1.0 :`G` 0.466324 :`A` 1.0) 3.0)
  (return))

(fn `UserConstructionScript`)