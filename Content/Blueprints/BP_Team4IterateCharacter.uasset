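; BP_Team4IterateCharacter is a player character that launches itself toward the cursor and manipulates its current tile.
; Left click, while alive, plays a flight animation and, after a cooldown, adds a velocity impulse toward the point under the cursor.
; A persistent debug trace draws the path, and releasing the button plays a crow call.
; Q, W, E and R move CurrentTile up or down and inflate or deflate its gap.
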(event `Key|LeftMouseButton`
  (params (Key :type "Key Structure"))
  (bind _returnvalue (`self.K2_GetActorLocation`))
  (bind _returnvalue_2 (`KismetSystemLibrary.GetGameTimeInSeconds`))
  (bind (_bblockinghit _binitialoverlap _time _distance _location _impactpoint) (`GameplayStatics.BreakHitResult` (`PlayerController.GetHitResultUnderCursorByChannel` (`GameplayStatics.GetPlayerController` 0) "TraceTypeQuery2" true)))
  ;[1 1 1] Grapple
  (:`Pressed`
    (if (not (`self.IsDead`))
      (`SkeletalMeshComponent.PlayAnimation` (`self.Mesh`) "/Game/Ravens_Crows/Animations/Common/Rav_C_Fly_Forward.Rav_C_Fly_Forward" false)
      (if (< (`self.LastTime`) (- _returnvalue_2 (`self.TimeToWait`)))
        (if true
          (`KismetSystemLibrary.LineTraceSingle` :`Start` _returnvalue :`End` _impactpoint :`TraceChannel` "TraceTypeQuery2" :`DrawDebugType` "Persistent")
          (`CharacterMovementComponent.AddImpulse` (`self.CharacterMovement`) (* (`KismetMathLibrary.GetDirectionUnitVector` _returnvalue _impactpoint) 2000.0) true)
          (set `self.LastTime` _returnvalue_2)))))
  (:`Released`
    (if (not (`self.IsDead`))
      (`GameplayStatics.PlaySoundAtLocation` "/Game/Sounds/crow_voice.crow_voice" (`SceneComponent.K2_GetComponentLocation` (`self.Mesh`)) (struct) 1.0 1.0 0.0 null null null))))

(event `Key|Q`
  (params (Key :type "Key Structure"))
  (:`Pressed`
    (`/Game/Blueprints/ByreaveBP_Tile.MovesUp` (`self.CurrentTile`))))

(event `Key|W`
  (params (Key :type "Key Structure"))
  (:`Pressed`
    (`/Game/Blueprints/ByreaveBP_Tile.MovesDown` (`self.CurrentTile`))))

(event `Key|E`
  (params (Key :type "Key Structure"))
  (:`Pressed`
    (`/Game/Blueprints/ByreaveBP_Tile.InflateGap` (`self.CurrentTile`))))

(event `Key|R`
  (params (Key :type "Key Structure"))
  (:`Pressed`
    (`/Game/Blueprints/ByreaveBP_Tile.DeflateGap` (`self.CurrentTile`))))

(fn `UserConstructionScript`)