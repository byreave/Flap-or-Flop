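; BP_HelpingShape is a trigger actor that smoothly lifts whatever overlaps it upward and slightly along world X.
; BeginPlay applies the helper material to its mesh.
; On overlap, it captures the actor's location, adds a fixed offset, and the SmoothMove timeline lerps the actor there without sweeping.
; IsPlayerActor compares against the player character but returns no result, so it does not restrict the move to the player.
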(event `self.ReceiveBeginPlay`
  (`PrimitiveComponent.SetMaterial` (`self.HelpingMesh`) 0 "/Game/Materials/MI_HelpingShapeMesh.MI_HelpingShapeMesh"))

(event `self.Trigger.OnComponentBeginOverlap`
  (params (OverlappedComponent :type "PrimitiveComponent Object Reference") (OtherActor :type "Actor Object Reference") (OtherComp :type "PrimitiveComponent Object Reference") (OtherBodyIndex :type Integer) (bFromSweep :type Boolean) (SweepResult :type "HitResult Structure (by ref)"))
  (set `self.OverlappedComponent` OverlappedComponent)
  (bind _output_get (set `self.OtherActor` OtherActor))
  (`self.Is Player Actor` _output_get)
  (bind _output_get_2 (set `self.Player Start` (`self.K2_GetActorLocation` (`self.OtherActor`))))
  (set `self.Player End` (`KismetMathLibrary.MakeVector` (+ (.x _output_get_2) 100.0) (.y _output_get_2) (+ (.z _output_get_2) 707.5)))
  (bind (_direction _driver) (`Timeline|SmoothMove`)
    (:`Update`
      (`self.K2_SetActorRelativeLocation` (`self.OtherActor`) (`KismetMathLibrary.VLerp` (`self.Player Start`) (`self.Player End`) _driver) false false))))

(fn `UserConstructionScript`)