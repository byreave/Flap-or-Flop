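; Infinite-terrain tile with an upper and lower obstacle around a gap, randomized in height and size on BeginPlay.
; Player overlaps register it as the character's current tile, add score once, request another tile from InfiniteTerrainGameMode on leaving, and destroy it.
; Touching the floor, roof or obstacles sets the character's IsDead.
; Clamped functions shift or resize the gap, and an Arrow supplies the attach transform; Lock and Unlock are empty.
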(event `self.LockingVolume.OnComponentBeginOverlap`
  (params (OverlappedComponent :type "PrimitiveComponent Object Reference") (OtherActor :type "Actor Object Reference") (OtherComp :type "PrimitiveComponent Object Reference") (OtherBodyIndex :type Integer) (bFromSweep :type Boolean) (SweepResult :type "HitResult Structure (by ref)"))
  ;[1 1 1] ForTesting
  (`self.Is Player Actor` OtherActor)
  (bind _asbp_team_4iterate_character (cast `/Game/Blueprints/BP_Team4IterateCharacter` (`GameplayStatics.GetPlayerCharacter` 0)))
  (set `/Game/Blueprints/BP_Team4IterateCharacter.CurrentTile` self _asbp_team_4iterate_character))

(event `self.DestoryVolume.OnComponentBeginOverlap`
  (params (OverlappedComponent :type "PrimitiveComponent Object Reference") (OtherActor :type "Actor Object Reference") (OtherComp :type "PrimitiveComponent Object Reference") (OtherBodyIndex :type Integer) (bFromSweep :type Boolean) (SweepResult :type "HitResult Structure (by ref)"))
  (`self.Is Player Actor` OtherActor)
  (`self.K2_DestroyActor`))

(event `self.LockingVolume.OnComponentEndOverlap`
  (params (OverlappedComponent :type "PrimitiveComponent Object Reference") (OtherActor :type "Actor Object Reference") (OtherComp :type "PrimitiveComponent Object Reference") (OtherBodyIndex :type Integer))
  (`self.Is Player Actor` OtherActor)
  (bind _asinfinite_terrain_game_mode (cast `/Game/InfiniteTerrainGameMode` (`GameplayStatics.GetGameMode`)))
  (`/Game/InfiniteTerrainGameMode.Spawn Tile` _asinfinite_terrain_game_mode))

(event `self.ReceiveBeginPlay`
  ;[1 1 1] Randomize the Gap
  (`SceneComponent.K2_SetRelativeLocation` (`self.BlockPos`) (`KismetMathLibrary.MakeVector` (.x (`SceneComponent.RelativeLocation` (`self.BlockPos`))) (.y (`SceneComponent.RelativeLocation` (`self.BlockPos`))) (`KismetMathLibrary.RandomFloatInRange` (`self.MinPos`) (`self.MaxPos`))) false false)
  (`self.RandomizeGap`))

(event `self.ScoreArea.OnComponentBeginOverlap`
  (params (OverlappedComponent :type "PrimitiveComponent Object Reference") (OtherActor :type "Actor Object Reference") (OtherComp :type "PrimitiveComponent Object Reference") (OtherBodyIndex :type Integer) (bFromSweep :type Boolean) (SweepResult :type "HitResult Structure (by ref)"))
  ;[1 1 1] Scores
  (`self.Is Player Actor` OtherActor)
  (if (not (`self.IsPassed`))
    (set `self.IsPassed` true)
    (bind _asinfinite_terrain_game_mode (cast `/Game/InfiniteTerrainGameMode` (`GameplayStatics.GetGameMode`)))
    (set `/Game/InfiniteTerrainGameMode.Scores` (+ (`/Game/InfiniteTerrainGameMode.Scores` _asinfinite_terrain_game_mode) 10.0) _asinfinite_terrain_game_mode)))

(event `self.Floor.OnComponentHit`
  (params (HitComponent :type "PrimitiveComponent Object Reference") (OtherActor :type "Actor Object Reference") (OtherComp :type "PrimitiveComponent Object Reference") (NormalImpulse :type "Vector Structure") (Hit :type "HitResult Structure (by ref)"))
  ;[1 1 1] Death Check
  (bind _asbp_team_4iterate_character (cast `/Game/Blueprints/BP_Team4IterateCharacter` OtherActor))
  (set `/Game/Blueprints/BP_Team4IterateCharacter.IsDead` true _asbp_team_4iterate_character))

(event `self.RoofDeathCheck.OnComponentBeginOverlap`
  (params (OverlappedComponent :type "PrimitiveComponent Object Reference") (OtherActor :type "Actor Object Reference") (OtherComp :type "PrimitiveComponent Object Reference") (OtherBodyIndex :type Integer) (bFromSweep :type Boolean) (SweepResult :type "HitResult Structure (by ref)"))
  ;[1 1 1] Death Check
  (bind _asbp_team_4iterate_character (cast `/Game/Blueprints/BP_Team4IterateCharacter` OtherActor))
  (set `/Game/Blueprints/BP_Team4IterateCharacter.IsDead` true _asbp_team_4iterate_character))

(event `self.DownMesh.OnComponentHit`
  (params (HitComponent :type "PrimitiveComponent Object Reference") (OtherActor :type "Actor Object Reference") (OtherComp :type "PrimitiveComponent Object Reference") (NormalImpulse :type "Vector Structure") (Hit :type "HitResult Structure (by ref)"))
  ;[1 1 1] Death Check
  (bind _asbp_team_4iterate_character (cast `/Game/Blueprints/BP_Team4IterateCharacter` OtherActor))
  (set `/Game/Blueprints/BP_Team4IterateCharacter.IsDead` true _asbp_team_4iterate_character))

(event `self.UpMesh.OnComponentHit`
  (params (HitComponent :type "PrimitiveComponent Object Reference") (OtherActor :type "Actor Object Reference") (OtherComp :type "PrimitiveComponent Object Reference") (NormalImpulse :type "Vector Structure") (Hit :type "HitResult Structure (by ref)"))
  ;[1 1 1] Death Check
  (bind _asbp_team_4iterate_character (cast `/Game/Blueprints/BP_Team4IterateCharacter` OtherActor))
  (set `/Game/Blueprints/BP_Team4IterateCharacter.IsDead` true _asbp_team_4iterate_character))

(fn `DeflateGap`
  (if (> (`self.CurrentGap`) (`self.MinGap`))
    (`SceneComponent.K2_AddLocalOffset` (`self.DownMesh`) (`KismetMathLibrary.MakeVector` 0.0 0.0 (`self.GapStep`)) false false)
    (`SceneComponent.K2_AddLocalOffset` (`self.UpMesh`) (`KismetMathLibrary.MakeVector` 0.0 0.0 (- 0.0 (`self.GapStep`))) false false)
    (set `self.CurrentGap` (- (`self.CurrentGap`) (* 2 (`self.GapStep`))))
    (else
      (`KismetSystemLibrary.PrintString` "Min Gap Hit"))))

(fn `Get Attach Location`
  (returns (`Attach Transform` :type "Transform Structure"))
  (return (`SceneComponent.K2_GetComponentToWorld` (`self.Arrow`))))

(fn `InflateGap`
  (if (< (`self.CurrentGap`) (`self.MaxGap`))
    (`SceneComponent.K2_AddLocalOffset` (`self.DownMesh`) (`KismetMathLibrary.MakeVector` 0.0 0.0 (- 0.0 (`self.GapStep`))) false false)
    (`SceneComponent.K2_AddLocalOffset` (`self.UpMesh`) (`KismetMathLibrary.MakeVector` 0.0 0.0 (`self.GapStep`)) false false)
    (set `self.CurrentGap` (+ (`self.CurrentGap`) (* 2 (`self.GapStep`))))
    (else
      (`KismetSystemLibrary.PrintString` "Max Gap Hit"))))

(fn `Lock`)

(fn `MovesDown`
  (if (> (.z (`SceneComponent.RelativeLocation` (`self.BlockPos`))) (`self.MinPos`))
    (`SceneComponent.K2_AddLocalOffset` (`self.BlockPos`) (`KismetMathLibrary.MakeVector` 0.0 0.0 (- 0.0 (`self.MoveStep`))) false false)))

(fn `MovesUp`
  (bind _blockpos (`self.BlockPos`))
  (if (< (.z (`SceneComponent.RelativeLocation` _blockpos)) (`self.MaxPos`))
    (`SceneComponent.K2_AddLocalOffset` _blockpos (`KismetMathLibrary.MakeVector` 0.0 0.0 (`self.MoveStep`)) false false)))

(fn `RandomizeGap`
  (locals (TempGap :type "Float (double-precision)"))
  (bind _output_get (set `local.TempGap` (`KismetMathLibrary.RandomFloatInRange` (`self.MinGap`) (`self.MaxGap`))))
  (`SceneComponent.K2_AddLocalOffset` (`self.UpMesh`) (`KismetMathLibrary.MakeVector` 0.0 0.0 (/ (- _output_get (`self.CurrentGap`)) 2.0)) false false)
  (`SceneComponent.K2_AddLocalOffset` (`self.DownMesh`) (`KismetMathLibrary.MakeVector` 0.0 0.0 (- 0.0 (/ (- (`local.TempGap`) (`self.CurrentGap`)) 2.0))) false false)
  (set `self.CurrentGap` (`local.TempGap`)))

(fn `Unlock`)

(fn `UserConstructionScript`)