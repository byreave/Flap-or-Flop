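; Bird character Blueprint with a cursor-aimed grapple-style dash and a steadily moving camera.
; Left click plays a forward-fly animation and, if the cooldown has elapsed, applies a velocity-change impulse toward the world point under the cursor.
; The accompanying line trace draws debug lines, but its result does not affect the movement.
; Tick offsets the CameraBoom along its local X axis at CameraSpeed, scaled by delta time.
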(event `Key|LeftMouseButton`
  (params (Key :type "Key Structure"))
  (bind _returnvalue (`self.K2_GetActorLocation`))
  (bind _returnvalue_2 (`KismetSystemLibrary.GetGameTimeInSeconds`))
  (bind (_bblockinghit _binitialoverlap _time _distance _location _impactpoint) (`GameplayStatics.BreakHitResult` (`PlayerController.GetHitResultUnderCursorByChannel` (`GameplayStatics.GetPlayerController` 0) "TraceTypeQuery1" true)))
  ;[1 1 1] Grapple
  (:`Pressed`
    (`SkeletalMeshComponent.PlayAnimation` (`self.Mesh`) "/Game/Ravens_Crows/Animations/Common/Rav_C_Fly_Forward.Rav_C_Fly_Forward" false)
    (if (< (`self.LastTime_1`) (- _returnvalue_2 (`self.TimeToWait_1`)))
      (if true
        (`KismetSystemLibrary.LineTraceSingle` :`Start` _returnvalue :`End` _impactpoint :`TraceChannel` "TraceTypeQuery1" :`DrawDebugType` "ForDuration")
        (`CharacterMovementComponent.AddImpulse` (`self.CharacterMovement`) (* (`KismetMathLibrary.GetDirectionUnitVector` _returnvalue _impactpoint) 2000.0) true)
        (set `self.LastTime_1` _returnvalue_2)))))

(event `self.ReceiveTick`
  (params (DeltaSeconds :type "Float (single-precision)"))
  (`SceneComponent.K2_AddLocalOffset` (`self.CameraBoom`) (`KismetMathLibrary.MakeVector` (* DeltaSeconds (`self.CameraSpeed`))) false false))

(fn `UserConstructionScript`)